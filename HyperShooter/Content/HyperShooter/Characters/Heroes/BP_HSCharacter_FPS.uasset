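; HyperShooter FPS hero character, handling input, weapon selection, hit reactions and the death-to-respawn cycle.
; Hard-coded keys drive crouch, zoom camera modes, grenade montages and nested FlipFlop weapon switching through a server update.
; BeginPlay creates dynamic materials for a dissolve-in, links pistol animation layers and equips the pistol.
; Death plays a directional montage, dissolves on blend-out and ragdolls, while the authority unpossesses, restarts the player and destroys the actor.
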(event Custom|Reverse%20Dissolve%20Multicast
  ;[1 1 1] Dissolve
  (bind _dissolve (Timeline|타임라인 ReverseFromEnd)
    (:Update
      (for _array_element (Variables|Default|GetDynamicMaterials)
        (Rendering|Material|SetScalarParameterValue _array_element "Dissolve" _dissolve :!class /Script/Engine.MaterialInstanceDynamic)))))

(event EventBeginPlay
  (bind _mesh (Variables|Character|GetMesh))
  ;[1 1 1] Begin Start
  (Utilities|FlowControl|Sequence
    (:then_0
      (for (_array_element _array_index) (Rendering|Material|GetMaterials (Variables|Character|GetMesh))
        (bind _returnvalue (Rendering|Material|CreateDynamicMaterialInstance _array_element "None" "None" :!class /Script/Engine.KismetMaterialLibrary))
        (bind _returnvalue_2 (Rendering|Material|CreateDynamicMaterialInstance _mesh _array_index _returnvalue "None" :!class /Script/Engine.PrimitiveComponent))
        (Rendering|Material|SetMaterial _mesh _array_index _returnvalue_2)
        (Utilities|Array|Add (Variables|Default|GetDynamicMaterials) _returnvalue_2)))
    (:then_1
      (CallFunction|ReverseDissolveMulticast)
      (Components|SkeletalMesh|AnimationBlueprintLinking|LinkAnimClassLayers (Variables|Character|GetMesh) "/Game/HyperShooter/Characters/Heroes/Animations/Pistol/ABP_Pistol.ABP_Pistol_C")
      (Utilities|FlowControl|Delay 0.5)
      (Class|HyperShooterCharacter|UpdateWeaponInfoServer "/Game/HyperShooter/Characters/Heroes/Weapon/Data/DA_Pistol.DA_Pistol"))))

(event EventTick
  (params (DeltaSeconds :type Float%20%28single-precision%29)))

(event EventPlayDeathMontage
  (params (hitDirection :type EHSHitDirection%20Enum :default "Front"))
  (bind _returnvalue (Pawn|GetController))
  (bind _mesh (Variables|Character|GetMesh))
  ;[1 1 1] Play Death Montage
  (Networking|SwitchHasAuthority
    (:Authority
      (bind _output_get (Variables|Default|SetCachedPC _returnvalue))
      (Pawn|UnPossess _returnvalue))
    (:Remote
      _))
  (switch Utilities|FlowControl|Switch|SwitchonEHSHitDirection hitDirection
    (:Front
      (Variables|Default|SetDeathMontage (.OutItem (Utilities|Array|Random (Variables|Default|GetFrontDeathMontages)))))
    (:Back
      (Variables|Default|SetDeathMontage "/Game/HyperShooter/Characters/Heroes/Mannequin/Animations/Actions/AM_MM_Death_Back_01.AM_MM_Death_Back_01"))
    (:Left
      (Variables|Default|SetDeathMontage "/Game/HyperShooter/Characters/Heroes/Mannequin/Animations/Actions/AM_MM_Death_Left_01.AM_MM_Death_Left_01"))
    (:Right
      (Variables|Default|SetDeathMontage "/Game/HyperShooter/Characters/Heroes/Mannequin/Animations/Actions/AM_MM_Death_Right_01.AM_MM_Death_Right_01")))
  (Animation|Montage|PlayMontage (Variables|Character|GetMesh) (Variables|Default|GetDeathMontage)
    (:OnCompleted
      (Collision|SetCollisionEnabled (Variables|Default|GetCapsuleComponent) "NoCollision")
      (Collision|SetCollisionEnabled _mesh "PhysicsOnly")
      (Physics|SetSimulatePhysics _mesh true)
      (Networking|SwitchHasAuthority
        (:Authority
          (Utilities|FlowControl|Delay 3.0)
          (Animation|Montage|MontageStop (Components|SkeletalMesh|GetAnimInstance (Variables|Character|GetMesh)) 0.0 0)
          (Class|GameModeBase|RestartPlayer (Game|GetGameMode) (Variables|Default|GetCachedPC))
          (Actor|DestroyActor))))
    (:OnBlendOut
      (bind _dissolve (Timeline|Dissolve PlayFromStart)
        (:Update
          (for _array_element (Variables|Default|GetDynamicMaterials)
            (Rendering|Material|SetScalarParameterValue _array_element "Dissolve" _dissolve :!class /Script/Engine.MaterialInstanceDynamic)))))))

(event EventPlayHitMontage
  (params (hitDirection :type EHSHitDirection%20Enum :default "Front"))
  ;[1 1 1] Play Hit Motnage
  (Development|PrintString (Utilities|String|EnumtoString hitDirection))
  (switch Utilities|FlowControl|Switch|SwitchonEHSHitDirection hitDirection
    (:Front
      (Variables|Default|SetHitMontage (.OutItem (Utilities|Array|Random (Variables|Default|GetFrontHitMontages)))))
    (:Back
      (Variables|Default|SetHitMontage "/Game/HyperShooter/Characters/Heroes/Mannequin/Animations/Actions/AM_MM_HitReact_Back_Lgt_01.AM_MM_HitReact_Back_Lgt_01"))
    (:Left
      (Variables|Default|SetHitMontage "/Game/HyperShooter/Characters/Heroes/Mannequin/Animations/Actions/AM_MM_HitReact_Left_Lgt_01.AM_MM_HitReact_Left_Lgt_01"))
    (:Right
      (Variables|Default|SetHitMontage "/Game/HyperShooter/Characters/Heroes/Mannequin/Animations/Actions/AM_MM_HitReact_Right_Lgt_01.AM_MM_HitReact_Right_Lgt_01")))
  (Animation|Montage|PlayMontage (Variables|Character|GetMesh) (Variables|Default|GetHitMontage)))

(event EventPossessed
  (params (NewController :type Controller%20Object%20Reference)))

(event Input|KeyboardEvents|Tab
  (params (Key :type Key%20Structure :default "None"))
  (:Pressed
    (Utilities|FlowControl|FlipFlop
      (:A
        (Class|HyperShooterCharacter|UpdateWeaponInfoServer "/Game/HyperShooter/Characters/Heroes/Weapon/Data/DA_Pistol.DA_Pistol"))
      (:B
        (Utilities|FlowControl|FlipFlop
          (:A
            (Class|HyperShooterCharacter|UpdateWeaponInfoServer "/Game/HyperShooter/Characters/Heroes/Weapon/Data/DA_Rifle.DA_Rifle"))
          (:B
            (Class|HyperShooterCharacter|UpdateWeaponInfoServer "/Game/HyperShooter/Characters/Heroes/Weapon/Data/DA_Shotgun.DA_Shotgun")))))))

(event Input|KeyboardEvents|LeftCtrl
  (params (Key :type Key%20Structure :default "None"))
  (:Pressed
    (Character|Crouch))
  (:Released
    (Character|UnCrouch)))

(event Input|MouseEvents|RightMouseButton
  (params (Key :type Key%20Structure :default "None"))
  (bind _charactermovement (Variables|Character|GetCharacterMovement))
  (bind _charactermovement_2 (Variables|Character|GetCharacterMovement))
  (:Pressed
    (Class|HSCameraModeComponent|SetCameraMode (Variables|Default|GetCameraModeComponent) "/Game/HyperShooter/CameraMode/BP_ZoomInCameraMode.BP_ZoomInCameraMode_C")
    (Variables|/Script/Engine.CharacterMovementComponent|SetbUseControllerDesiredRotation _charactermovement true)
    (Variables|/Script/Engine.CharacterMovementComponent|SetbOrientRotationToMovement _charactermovement false))
  (:Released
    (Class|HSCameraModeComponent|SetCameraMode (Variables|Default|GetCameraModeComponent) "/Game/HyperShooter/CameraMode/BP_DefaultCameraMode.BP_DefaultCameraMode_C")
    (Variables|/Script/Engine.CharacterMovementComponent|SetbUseControllerDesiredRotation _charactermovement_2 true)
    (Variables|/Script/Engine.CharacterMovementComponent|SetbOrientRotationToMovement _charactermovement_2 false)))

(event Input|KeyboardEvents|NumPadOne
  (params (Key :type Key%20Structure :default "None")))

(event Input|KeyboardEvents|1
  (params (Key :type Key%20Structure :default "None"))
  (:Pressed
    (Animation|Montage|PlayMontage (Variables|Character|GetMesh) "/Game/HyperShooter/Characters/Heroes/Animations/Grenade/AM_Throw_Grenade_Loop.AM_Throw_Grenade_Loop")))

(event Input|KeyboardEvents|2
  (params (Key :type Key%20Structure :default "None"))
  (:Pressed
    (Animation|Montage|PlayMontage (Variables|Character|GetMesh) "/Game/HyperShooter/Characters/Heroes/Animations/Grenade/AM_Throw_Grenade.AM_Throw_Grenade")))

(fn ConstructionScript)
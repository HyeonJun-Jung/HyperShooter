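; BP_HeroPlayerController is the hero player controller Blueprint for HyperShooter, and its only live logic is a debug key.
; Pressing P casts player state index 0 to HSPlayerState_Session and prints that player's team color and name.
; An unconnected chain would print the UserInfos count from HSGameState_Session, and BeginPlay, Tick and the construction script are empty.
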(event EventBeginPlay)

(event EventTick
  (params (DeltaSeconds :type Float%20%28single-precision%29)))

(event Input|KeyboardEvents|P
  (params (Key :type Key%20Structure :default "None"))
  (:Pressed
    (bind _ashsplayer_state_session (Utilities|Casting|CastToHSPlayerState_Session (Game|GetPlayerState 0)))
    (Development|PrintString (Utilities|String|EnumtoString (.TeamColor (Utilities|Struct|BreakUserInfo (Variables|/Script/HyperShooter.HSPlayerState_Session|GetPlayerInfo _ashsplayer_state_session)))))
    (Development|PrintString (Utilities|String|ToString(Name) (.PlayerName (Utilities|Struct|BreakUserInfo (Variables|/Script/HyperShooter.HSPlayerState_Session|GetPlayerInfo _ashsplayer_state_session)))))))

(fn ConstructionScript)